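; BP_BaseObject is a base Blueprint for damageable objects.
; On AnyDamage it subtracts damage from Life while not yet Dead, and at zero or below sets Dead and calls ObjectHandleDeath.
; ObjectHandleDeath only prints an override reminder, leaving the death behavior to child classes.
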(event `self.ReceiveAnyDamage`
  (params (Damage :type "Float (single-precision)") (DamageType :type "DamageType Object Reference") (InstigatedBy :type "Controller Object Reference") (DamageCauser :type "Actor Object Reference"))
  (if (not (`self.Dead`))
    (set `self.Life` (- (`self.Life`) Damage))
    (if (<= (`self.Life`) 0.0)
      (set `self.Dead` true)
      (`self.ObjectHandleDeath`))))

(event `ObjectHandleDeath`
  (`KismetSystemLibrary.PrintString` "Override ObjectHandleDeath"))

(fn `UserConstructionScript`)