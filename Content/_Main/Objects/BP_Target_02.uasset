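; BP_Target_02 is a destructible target object that breaks apart when its death is handled.
; On ObjectHandleDeath it plays a water ball hit particle effect at its location, spawns a Target_02_Fracture actor at its static mesh's transform, then destroys itself.
; Breakage is done by swapping in that separate fracture actor, and the file has no damage logic or other active events of its own.
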(event `self.ObjectHandleDeath`
  (`GameplayStatics.SpawnEmitterAtLocation` "/Game/FXVarietyPack/Particles/P_ky_waterBallHit.P_ky_waterBallHit" (`self.K2_GetActorLocation`))
  (`|SpawnActorFromClass` "/Game/_Main/Objects/Target_02_Fracture.Target_02_Fracture_C" (`SceneComponent.K2_GetComponentToWorld` (`self.StaticMesh`)) "Undefined" "MultiplyWithRoot" null null)
  (`self.K2_DestroyActor`))

(fn `UserConstructionScript`
  (`parent.UserConstructionScript`))