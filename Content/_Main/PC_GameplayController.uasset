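; Gameplay player controller that owns the HUD and toggles the in-game menu.
; On BeginPlay it adds the gameplay input mapping, creates the HUD and registers itself with the game mode.
; Events relay interact text, health, ammo, crosshair, level timer and death screen updates to the HUD.
; The menu action creates or removes the menu widget, switching input mode and cursor, as the death screen also does.
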(event `EnhancedInput|/Game/_Main/Inputs/InputActions/IA_InGameMenu`
  (params (ActionValue :type Boolean) (ElapsedSeconds :type "Float (double-precision)") (TriggeredSeconds :type "Float (double-precision)") (InputAction :type "InputAction Object Reference" :default "/Game/_Main/Inputs/InputActions/IA_InGameMenu.IA_InGameMenu"))
  (:`Started`
    (if (`self.InMenu`)
      (set `self.InMenu` true)
      (`Widget.RemoveFromParent` (`self.w_Menu`))
      (`WidgetBlueprintLibrary.SetInputMode_GameOnly` self)
      (set `self.bShowMouseCursor` false)
      (set `self.InMenu` false)
      (else
        (bind _returnvalue (`|CreateWidget` "/Game/_Main/UI/W_InGameMenu.W_InGameMenu_C" self))
        (bind _output_get (set `self.w_Menu` _returnvalue))
        (`UserWidget.AddToViewport` _output_get 0)
        (set `self.bShowMouseCursor` true)
        (`WidgetBlueprintLibrary.SetInputMode_GameAndUIEx` self (`self.w_Menu`) "DoNotLock" false)
        (set `self.InMenu` true)))))

(event `self.ReceiveBeginPlay`
  (bind _returnvalue (subsystem `EnhancedInputLocalPlayerSubsystem`))
  (`/Engine/EditorBlueprintResources/StandardMacros.IsValid` _returnvalue
    (:`Is Valid`
      (`EnhancedInputSubsystemInterface.AddMappingContext` _returnvalue "/Game/_Main/Inputs/IMC_Gameplay.IMC_Gameplay" 0 (struct))
      (bind _returnvalue_2 (`|CreateWidget` "/Game/_Main/UI/W_Hud.W_Hud_C" self))
      (bind _output_get (set `self.Hud` _returnvalue_2))
      (`UserWidget.AddToViewport` _output_get 0)
      (`WidgetBlueprintLibrary.SetInputMode_GameOnly` self)
      (set `self.bShowMouseCursor` false)
      (message `/Game/_Main/Interfaces/INT_GameMode.AddPlayerControllerToGameMode` (`GameplayStatics.GetGameMode`) self))))

(event `/Game/_Main/Interfaces/INT_PlayerController.SetInteractText`
  (params (TextToShow :type Text) (Visibility :type "ESlateVisibility Enum" :default "Visible"))
  (bind _hud (`self.Hud`)
    (:`then`
      (`/Game/_Main/UI/W_Hud.UpdateInteractText` _hud TextToShow Visibility))
    (:`else`)))

(event `/Game/_Main/Interfaces/INT_PlayerController.UpdateHealthUI`
  (params (HealthPercent :type "Float (double-precision)"))
  (bind _hud (`self.Hud`)
    (:`then`
      (`/Game/_Main/UI/W_Hud.UpdateHealth` _hud HealthPercent))
    (:`else`)))

(event `/Game/_Main/Interfaces/INT_PlayerController.UpdateAmmoUI`
  (params (WeaponName :type Text) (CurrentAmmo :type Integer) (TotalAmmo :type Integer))
  (bind _hud (`self.Hud`)
    (:`then`
      (`/Game/_Main/UI/W_Hud.UpdateAmmo` _hud WeaponName CurrentAmmo TotalAmmo))
    (:`else`)))

(event `/Game/_Main/Interfaces/INT_PlayerController.ShowPlayerDeathScreen`
  (`WidgetBlueprintLibrary.SetInputMode_GameAndUIEx` self (`self.Hud`) "LockAlways" false)
  (set `self.bShowMouseCursor` true)
  (bind _hud (`self.Hud`)
    (:`then`
      (`/Game/_Main/UI/W_Hud.ShowDeathUI` _hud))
    (:`else`)))

(event `/Game/_Main/Interfaces/INT_PlayerController.UpdateLevelText`
  (params (LevelTimer :type Text))
  (bind _hud (`self.Hud`)
    (:`then`
      (`/Game/_Main/UI/W_Hud.SetLevelTimer` _hud LevelTimer))
    (:`else`)))

(event `/Game/_Main/Interfaces/INT_PlayerController.UpdateCrosshair`
  (params (ChImage :type "Texture2D Object Reference") (Visibility :type "ESlateVisibility Enum" :default "Visible"))
  (bind _hud (`self.Hud`)
    (:`then`
      (`/Game/_Main/UI/W_Hud.UpdateCrosshair` _hud ChImage Visibility))
    (:`else`)))

(fn `UserConstructionScript`)