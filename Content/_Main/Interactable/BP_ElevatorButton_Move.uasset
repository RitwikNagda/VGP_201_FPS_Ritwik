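; An interactable elevator button that moves an assigned floor actor to a target location, starting out unusable at BeginPlay.
; When used while not in use, it lerps the floor from its current position to the call location through a timeline, or prints a warning if no floor is assigned.
; When the move finishes, it reveals and enables a linked button, then hides itself.
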(event `self.ReceiveBeginPlay`
  (`parent.ReceiveBeginPlay`)
  (set `self.CanUse` false))

(event `self.UseInteractable`
  (bind _buttontoshow (`self.ButtonToShow`))
  (if (not (`self.InUse`))
    (set `self.InUse` false)
    (`self.FloorToMove`
      (:`then`
        (set `self.Floor Start` (`self.K2_GetActorLocation` (`self.FloorToMove`)))
        (bind (_direction _floordelta) (`Timeline|FloorMoveTimeline` :!via `PlayFromStart`)
          (:`Update`
            (`self.K2_SetActorLocation` (`self.FloorToMove`) (`KismetMathLibrary.VLerp` (`self.Floor Start`) (`self.CallToLocation`) _floordelta) false false))
          (:`Finished`
            (`self.SetActorHiddenInGame` _buttontoshow false)
            (set `/Game/_Main/Interactable/BP_InteractableBase.CanUse` true _buttontoshow)
            (set `/Game/_Main/Interactable/BP_ElevatorButton_CallDown.InUse` false _buttontoshow)
            (`self.SetActorHiddenInGame` true))))
      (:`else`
        (`KismetSystemLibrary.PrintString` "Missing Floor to call")))))

(fn `UserConstructionScript`
  (`parent.UserConstructionScript`))