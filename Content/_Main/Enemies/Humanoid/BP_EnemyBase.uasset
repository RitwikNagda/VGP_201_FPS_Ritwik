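; Base humanoid enemy that registers with the game mode, patrols linked points and reacts to a seen player.
; SetPlayerTarget branches on EnemyMainDecision: chase, shoot, or flee to a random nearby BP_HidingSpot.
; Line traces gate hitscan damage and validate hiding spots; losing line of sight while shooting moves it toward the player's position.
; Lethal damage broadcasts EnemyKilled, detaches the controller and ragdolls the body.
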(event `self.ReceiveBeginPlay`
  (`parent.ReceiveBeginPlay`)
  (message `/Game/_Main/Interfaces/INT_GameMode.AddEnemy` (`GameplayStatics.GetGameMode`) self)
  (set `self.ShouldPatrol` true)
  (set `CharacterMovementComponent.MaxWalkSpeed` (`self.WalkSpeed`) (`self.CharacterMovement`))
  (`self.Patrol`))

(event `Patrol`
  (if (`self.ShouldPatrol`)
    (`self.SetActorTickEnabled` false)
    (set `CharacterMovementComponent.MaxWalkSpeed` (`self.WalkSpeed`) (`self.CharacterMovement`))
    (bind _patrolpoint (`self.PatrolPoint`)
      (:`then`
        (`|AIMoveTo` self (0.0 0.0 0.0) _patrolpoint
          (:`OnSuccess`
            (set `self.PatrolPoint` (`/Game/_Main/Enemies/BP_PetrolPoints.NextPetrolPoint` (`self.PatrolPoint`)))
            (`KismetSystemLibrary.Delay` (`KismetMathLibrary.RandomFloatInRange` 1.5 4.0))
            (`self.Patrol`))))
      (:`else`))))

(event `/Game/_Main/Interfaces/INT_EnemyCharacter.SetPlayerTarget`
  (params (PlayerReferance :type "/Game/_Main/Player/BP_Player Object Reference") (`Seen?` :type Boolean))
  (set `self.Player Referance` PlayerReferance)
  (if `Seen?`
    (set `self.ShouldPatrol` false)
    (switch `/Game/_Main/Enemies/Humanoid/E_EnemyMainDecision` (`self.EnemyMainDecision`)
      (:`NewEnumerator1`
        (if (not (`self.isRunHide`))
          (set `self.ShouldPatrol` false)
          (`self.RunHide`)))
      (:`NewEnumerator2`
        (set `self.ShouldChase` true)
        (`self.Chase`))
      (:`NewEnumerator3`
        (set `self.ShouldShoot` true)
        (`self.ShootAtPlayer`)))))

(event `self.ReceiveTick`
  (params (DeltaSeconds :type "Float (single-precision)"))
  (bind (_returnvalue_roll _returnvalue_pitch _returnvalue_yaw) (`KismetMathLibrary.BreakRotator` (`KismetMathLibrary.FindLookAtRotation` (`self.K2_GetActorLocation`) (`self.K2_GetActorLocation` (`self.Player Referance`)))))
  (`self.Player Referance`
    (:`then`
      (`self.K2_SetActorRotation` (`KismetMathLibrary.MakeRotator` 0.0 0.0 _returnvalue_yaw)))
    (:`else`
      (`self.SetActorTickEnabled` false))))

(event `Chase`
  (if (`self.ShouldChase`)
    (bind _player_referance (`self.Player Referance`)
      (:`then`
        (set `CharacterMovementComponent.MaxWalkSpeed` (`self.ChaseSpeed`) (`self.CharacterMovement`))
        (`|AIMoveTo` self (0.0 0.0 0.0) _player_referance))
      (:`else`
        (set `self.ShouldPatrol` true)
        (set `self.ShouldChase` false)
        (`self.Patrol`)))))

(event `ShootAtPlayer`
  (bind (_returnvalue_roll _returnvalue_pitch _returnvalue_yaw) (`KismetMathLibrary.BreakRotator` (`KismetMathLibrary.FindLookAtRotation` (`self.K2_GetActorLocation`) (`self.K2_GetActorLocation` (`self.Player Referance`)))))
  (`self.Player Referance`
    (:`then`
      (`|ExecutionSequence`
        (:`then_0`
          (`/Engine/EditorBlueprintResources/StandardMacros.DoOnce` false
            (:`Completed`
              (set `self.StartRotation` (`self.K2_GetActorRotation`))
              (bind (_direction _playerfacedelta) (`Timeline|FacePlayer` :!via `PlayFromStart`)
                (:`Update`
                  (bind (_returnvalue_roll_2 _returnvalue_pitch_2 _returnvalue_yaw_2) (`KismetMathLibrary.BreakRotator` (`KismetMathLibrary.RLerp` (`self.StartRotation`) (`KismetMathLibrary.MakeRotator` 0.0 0.0 _returnvalue_yaw) _playerfacedelta)))
                  (`self.K2_SetActorRotation` (`KismetMathLibrary.MakeRotator` 0.0 0.0 _returnvalue_yaw_2)))
                (:`Finished`
                  (`self.SetActorTickEnabled` true))))))
        (:`then_1`
          (if (`self.ShouldShoot`)
            (bind (_outhit _returnvalue) (`KismetSystemLibrary.LineTraceSingleForObjects` :`Start` (`self.K2_GetActorLocation`) :`End` (`self.K2_GetActorLocation` (`self.Player Referance`)) :`ObjectTypes` (`|MakeArray` "ObjectTypeQuery3" "ObjectTypeQuery1" "ObjectTypeQuery2" :!type "EObjectTypeQuery Enum") :`DrawDebugType` "ForDuration" :`DrawTime` 10.0))
            (if _returnvalue
              (bind (_bblockinghit _binitialoverlap _time _distance _location _impactpoint _normal _impactnormal _physmat _hitactor) (`GameplayStatics.BreakHitResult` _outhit))
              (if (`self.ActorHasTag` _hitactor "Player")
                (`GameplayStatics.ApplyDamage` _hitactor 5.0)
                (`KismetSystemLibrary.Delay` (`self.TimeBetweenShoots`))
                (`self.ShootAtPlayer`)
                (else
                  (`|AIMoveTo` self (`self.K2_GetActorLocation` (`self.Player Referance`)) null
                    (:`then`
                      (bind _returnvalue_2 (`KismetSystemLibrary.K2_SetTimerDelegate` (delegate `LookForPlayer`) 0.25))
                      (set `self.LookForPlayerHandle` _returnvalue_2))
                    (:`OnSuccess`
                      (set `self.ShouldShoot` false)
                      (`self.StopLookForPlayer`)
                      (set `self.ShouldPatrol` true)
                      (`self.Patrol`))))))))))
    (:`else`
      (set `self.ShouldPatrol` true)
      (`self.Patrol`))))

(event `LookForPlayer`
  (`self.Player Referance`
    (:`then`
      (bind (_outhit _returnvalue) (`KismetSystemLibrary.LineTraceSingleForObjects` :`Start` (`self.K2_GetActorLocation`) :`End` (`self.K2_GetActorLocation` (`self.Player Referance`)) :`ObjectTypes` (`|MakeArray` "ObjectTypeQuery3" "ObjectTypeQuery1" "ObjectTypeQuery2" :!type "EObjectTypeQuery Enum") :`DrawDebugType` "ForDuration" :`DrawTime` 10.0))
      (if _returnvalue
        (if (`self.ActorHasTag` (`.HitActor` (`GameplayStatics.BreakHitResult` _outhit)) "Player")
          (`self.StopLookForPlayer`)
          (`self.ShootAtPlayer`))))
    (:`else`)))

(event `StopLookForPlayer`
  (`KismetSystemLibrary.K2_ClearAndInvalidateTimerHandle` (`self.LookForPlayerHandle`)))

(event `RunHide`
  (set `self.isRunHide` true)
  (`KismetArrayLibrary.Array_Clear` (`self.HidingPoints`))
  (bind _outactors (`GameplayStatics.GetAllActorsOfClass` "/Game/_Main/Enemies/BP_HidingSpot.BP_HidingSpot_C"))
  (for _array_element _outactors
    (if (not (> (`self.GetDistanceTo` _array_element) (`self.HidingSpotDistance`)))
      (`KismetArrayLibrary.Array_AddUnique` (`self.HidingPoints`) _array_element)))
  (`self.Hide`))

(event `Hide`
  (if (> (`KismetArrayLibrary.Array_Length` (`self.HidingPoints`)) 0)
    (set `self.CurrentHideSpot` (`KismetArrayLibrary.Array_Random` (`self.HidingPoints`)))
    (`|AIMoveTo` self (0.0 0.0 0.0) (`self.CurrentHideSpot`)
      (:`OnSuccess`
        (bind (_outhit _returnvalue) (`KismetSystemLibrary.LineTraceSingleForObjects` :`Start` (`self.K2_GetActorLocation`) :`End` (`self.K2_GetActorLocation` (`self.Player Referance`)) :`ObjectTypes` (`|MakeArray` "ObjectTypeQuery3" "ObjectTypeQuery1" "ObjectTypeQuery2" :!type "EObjectTypeQuery Enum") :`DrawDebugType` "ForDuration" :`DrawTime` 10.0))
        (if _returnvalue
          (if (`self.ActorHasTag` (`.HitActor` (`GameplayStatics.BreakHitResult` _outhit)) "Player")
            (`KismetArrayLibrary.Array_RemoveItem` (`self.HidingPoints`) (`self.CurrentHideSpot`))
            (`self.Hide`)
            (else
              (`KismetSystemLibrary.Delay` 1.0)
              (set `self.isRunHide` false)
              (set `self.ShouldPatrol` true)
              (`self.Patrol`))))))
    (else
      (`self.RunHide`))))

(event `self.ReceiveAnyDamage`
  (params (Damage :type "Float (single-precision)") (DamageType :type "DamageType Object Reference") (InstigatedBy :type "Controller Object Reference") (DamageCauser :type "Actor Object Reference"))
  (if (not (`self.IsDead`))
    (set `self.CurrentHealth` (- (`self.CurrentHealth`) Damage))
    (if (<= (`self.CurrentHealth`) 0.0)
      (set `self.IsDead` true)
      (`self.EnemyKilled` self)
      (`self.HandleDeath`))))

(event `HandleDeath`
  (`MovementComponent.StopMovementImmediately` (`self.CharacterMovement`))
  (`self.DetachFromControllerPendingDestroy`)
  (set `self.ShouldPatrol` false)
  (set `self.ShouldShoot` false)
  (set `self.isRunHide` false)
  (set `self.ShouldChase` false)
  (set `self.Player Referance` null)
  (`PrimitiveComponent.SetCollisionProfileName` (`self.Mesh`) "ragdoll" true)
  (`PrimitiveComponent.SetCollisionProfileName` (`self.CapsuleComponent`) "ragdoll" true)
  (`PrimitiveComponent.SetSimulatePhysics` (`self.Mesh`) true))

(fn `GetEnemyCharacterReferance`
  (returns (EnemyBaseReferance :type "/Game/_Main/Enemies/Humanoid/BP_EnemyBase Object Reference"))
  (return self))

(fn `UserConstructionScript`
  (`parent.UserConstructionScript`))