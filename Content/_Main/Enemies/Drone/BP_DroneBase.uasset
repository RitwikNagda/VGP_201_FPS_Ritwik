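; Base enemy drone that patrols, chases the player and explodes on contact, dealing damage.
; It follows linked patrol points with AIMoveTo, using timelines to smooth yaw turns between states.
; Separate spheres detect the player, end the chase by moving to the player's exit location before resuming patrol, and trigger the explosion.
; Depleted health or detonation spawns an effect, rolls a chance to drop all listed items, and destroys it.
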(event `self.ReceiveBeginPlay`
  (set `self.DroneState` "NewEnumerator0")
  (`self.Patrol`)
  (message `/Game/_Main/Interfaces/INT_GameMode.AddEnemy` (`GameplayStatics.GetGameMode`) self))

(event `Patrol`
  (`self.PetrolPoint`
    (:`then`
      (switch `/Game/_Main/Enemies/Drone/E_DroneState` (`self.DroneState`)
        (:`NewEnumerator0`
          (`|AIMoveTo` self (0.0 0.0 0.0) (`self.PetrolPoint`)
            (:`then`
              (set `self.PetrolPoint` (`/Game/_Main/Enemies/BP_PetrolPoints.NextPetrolPoint` (`self.PetrolPoint`)))
              (set `self.PreTurnRotation` (`self.K2_GetActorRotation`))
              (bind (_direction _rotatedelta) (`Timeline|RotateTimeline` :!via `PlayFromStart`)
                (:`Update`
                  (bind (_returnvalue_roll _returnvalue_pitch _returnvalue_yaw) (`KismetMathLibrary.BreakRotator` (`KismetMathLibrary.RLerp` (`self.PreTurnRotation`) (`KismetMathLibrary.FindLookAtRotation` (`self.K2_GetActorLocation`) (`self.K2_GetActorLocation` (`self.PetrolPoint`))) _rotatedelta true)))
                  (`self.K2_SetActorRotation` (`KismetMathLibrary.MakeRotator` 0.0 0.0 _returnvalue_yaw)))
                (:`Finished`
                  (`KismetSystemLibrary.Delay` (`KismetMathLibrary.RandomFloatInRange` 0.5 1.5))
                  (switch `/Game/_Main/Enemies/Drone/E_DroneState` (`self.DroneState`)
                    (:`NewEnumerator0`
                      (`self.Patrol`))))))))))
    (:`else`)))

(event `self.ReceiveTick`
  (params (DeltaSeconds :type "Float (single-precision)"))
  (bind (_returnvalue_roll _returnvalue_pitch _returnvalue_yaw) (`KismetMathLibrary.BreakRotator` (`KismetMathLibrary.FindLookAtRotation` (`self.K2_GetActorLocation`) (`self.K2_GetActorLocation` (`self.PlayerTarget`)))))
  (`self.PlayerTarget`
    (:`then`
      (switch `/Game/_Main/Enemies/Drone/E_DroneState` (`self.DroneState`)
        (:`NewEnumerator0`
          (`self.SetActorTickEnabled` false))
        (:`NewEnumerator1`
          (`self.K2_SetActorRotation` (`KismetMathLibrary.MakeRotator` 0.0 0.0 _returnvalue_yaw)))))
    (:`else`
      (`self.SetActorTickEnabled` false))))

(event `Chase`
  (switch `/Game/_Main/Enemies/Drone/E_DroneState` (`self.DroneState`)
    (:`NewEnumerator1`
      (`|AIMoveTo` self (0.0 0.0 0.0) (`self.PlayerTarget`)
        (:`OnSuccess`
          (switch `/Game/_Main/Enemies/Drone/E_DroneState` (`self.DroneState`)
            (:`NewEnumerator1`
              (`KismetSystemLibrary.Delay` 0.2)
              (`self.Chase`))))))))

(event `self.FindPlayerSphere.OnComponentBeginOverlap`
  (params (OverlappedComponent :type "PrimitiveComponent Object Reference") (OtherActor :type "Actor Object Reference") (OtherComp :type "PrimitiveComponent Object Reference") (OtherBodyIndex :type Integer) (bFromSweep :type Boolean) (SweepResult :type "HitResult Structure (by ref)"))
  (if (`self.ActorHasTag` OtherActor "Player")
    (bind _playerreferance (message `/Game/_Main/Interfaces/INT_Player.GetPlayerReferance` OtherActor))
    (`/Engine/EditorBlueprintResources/StandardMacros.IsValid` _playerreferance
      (:`Is Valid`
        (set `self.PlayerTarget` _playerreferance)
        (`MovementComponent.StopMovementImmediately` (`self.FloatingPawnMovement`))
        (set `self.DroneState` "NewEnumerator1")
        (set `self.PreTurnRotation` (`self.K2_GetActorRotation`))
        (bind (_direction _newtrack_1) (`Timeline|Chase Turn` :!via `PlayFromStart`)
          (:`Update`
            (bind (_returnvalue_roll _returnvalue_pitch _returnvalue_yaw) (`KismetMathLibrary.BreakRotator` (`KismetMathLibrary.RLerp` (`self.PreTurnRotation`) (`KismetMathLibrary.FindLookAtRotation` (`self.K2_GetActorLocation`) (`self.K2_GetActorLocation` (`self.PlayerTarget`))) _newtrack_1 true)))
            (`self.K2_SetActorRotation` (`KismetMathLibrary.MakeRotator` 0.0 0.0 _returnvalue_yaw)))
          (:`Finished`
            (`self.SetActorTickEnabled` false)
            (`self.Chase`)))))))

(event `self.LosePlayerSphere.OnComponentEndOverlap`
  (params (OverlappedComponent :type "PrimitiveComponent Object Reference") (OtherActor :type "Actor Object Reference") (OtherComp :type "PrimitiveComponent Object Reference") (OtherBodyIndex :type Integer))
  (if (`self.ActorHasTag` OtherActor "Player")
    (set `self.PlayerTarget` null)
    (set `self.DroneState` "NewEnumerator0")
    (`MovementComponent.StopMovementImmediately` (`self.FloatingPawnMovement`))
    (`|AIMoveTo` self (`self.K2_GetActorLocation` OtherActor) null
      (:`OnSuccess`
        (set `self.PreTurnRotation` (`self.K2_GetActorRotation`))
        (bind (_direction _turndelta) (`Timeline|PatrolTurn` :!via `PlayFromStart`)
          (:`Update`
            (bind (_returnvalue_roll _returnvalue_pitch _returnvalue_yaw) (`KismetMathLibrary.BreakRotator` (`KismetMathLibrary.RLerp` (`self.PreTurnRotation`) (`KismetMathLibrary.FindLookAtRotation` (`self.K2_GetActorLocation`) (`self.K2_GetActorLocation` (`self.PetrolPoint`))) _turndelta true)))
            (`self.K2_SetActorRotation` (`KismetMathLibrary.MakeRotator` 0.0 0.0 _returnvalue_yaw)))
          (:`Finished`
            (`KismetSystemLibrary.Delay` 0.25)
            (`self.Patrol`)))))))

(event `self.ExplodeSphere.OnComponentBeginOverlap`
  (params (OverlappedComponent :type "PrimitiveComponent Object Reference") (OtherActor :type "Actor Object Reference") (OtherComp :type "PrimitiveComponent Object Reference") (OtherBodyIndex :type Integer) (bFromSweep :type Boolean) (SweepResult :type "HitResult Structure (by ref)"))
  (if (`self.ActorHasTag` OtherActor "Player")
    (`GameplayStatics.ApplyDamage` OtherActor (`self.ExplodeDamage`))
    (`self.DestroyDrone`)))

(event `self.ReceiveAnyDamage`
  (params (Damage :type "Float (single-precision)") (DamageType :type "DamageType Object Reference") (InstigatedBy :type "Controller Object Reference") (DamageCauser :type "Actor Object Reference"))
  (set `self.Health` (- (`self.Health`) Damage))
  (if (<= (`self.Health`) 0.0)
    (`self.DestroyDrone`)))

(event `DestroyDrone`
  (bind _skeletalmesh (`self.SkeletalMesh`))
  (`GameplayStatics.SpawnEmitterAtLocation` "/Game/_Main/Enemies/Drone/DroneExplode.DroneExplode" (`SceneComponent.K2_GetComponentLocation` _skeletalmesh) (`SceneComponent.K2_GetComponentRotation` _skeletalmesh))
  (`self.DropItems`)
  (`self.K2_DestroyActor`))

(event `DropItems`
  (if (`self.F_DropItemChance`)
    (`self.F_DropItem`)))

(fn `F_DropItem`
  (bind _itemstodrop (`self.ItemsToDrop`))
  (if (> (`KismetArrayLibrary.Array_Length` _itemstodrop) 0)
    (for _array_element _itemstodrop
      (`|SpawnActorFromClass` _array_element (`KismetMathLibrary.MakeTransform` (`self.K2_GetActorLocation`)) "AdjustIfPossibleButAlwaysSpawn" "MultiplyWithRoot" null null)))
  (return))

(fn `F_DropItemChance`
  (returns (DropItem :type Boolean))
  (return (<= (`KismetMathLibrary.RandomFloatInRange` 0.0 100.0) (`self.PercentToDrop`))))

(fn `UserConstructionScript`)