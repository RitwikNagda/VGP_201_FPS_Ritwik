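; Gameplay game mode that runs level objectives, an optional countdown and the carry-over of player weapons and ammo between levels.
; BeginPlay reads rules from BP_LevelType, restores the SG_GameSave, retrying until the registered PlayerController is valid, and starts any timer, which kills the player at zero.
; Emptying the registered enemy list or reaching the level end, depending on level type, saves and opens the next map.
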(event `LoadPlayerData`
  (bind _player_referance (`self.Player Referance`))
  (bind _player_referance_2 (`self.Player Referance`))
  (bind _savegamename (message `/Game/_Main/Interfaces/INT_GameInstance.GetSaveGameName` (`GameplayStatics.GetGameInstance`)))
  (bind _returnvalue (`GameplayStatics.DoesSaveGameExist` _savegamename))
  (if _returnvalue
    (bind _player_controller (`self.Player Controller` :!label _label)
      (:`then`
        (bind _playerreferance (message `/Game/_Main/Interfaces/INT_Player.GetPlayerReferance` (`Controller.K2_GetPawn` _player_controller)))
        (set `self.Player Referance` _playerreferance)
        (bind _returnvalue_2 (`GameplayStatics.LoadGameFromSlot` _savegamename))
        (bind _output_get (set `self.LoadGameData` (cast `/Game/_Main/SG_GameSave` _returnvalue_2 :!pure true)))
        (set `/Game/_Main/Player/BP_Player.OwnedWeaponCurrentAmmo` (`/Game/_Main/SG_GameSave.CurrentAmmo` _output_get) _player_referance_2)
        (set `/Game/_Main/Player/BP_Player.OwnedWeaponTotalAmmo` (`/Game/_Main/SG_GameSave.TotalAmmo` _output_get) _player_referance_2)
        (set `/Game/_Main/Player/BP_Player.OwnedWeapons` (`/Game/_Main/SG_GameSave.OwnedWeapons` _output_get) _player_referance_2)
        (bind _returnvalue_3 (`|SpawnActorFromClass` (`/Game/_Main/SG_GameSave.CurrentlyHeldWeapon` _output_get) (`KismetMathLibrary.MakeTransform` (`self.K2_GetActorLocation` _player_referance_2)) "AlwaysSpawn" "MultiplyWithRoot" null null))
        (bind _output_get_2 (set `/Game/_Main/Player/BP_Player.HeldWeapon` _returnvalue_3 _player_referance))
        (`SceneComponent.K2_AttachToComponent` (`/Game/_Main/Weapon/BP_EQ_WeaponBase.SkeletalMesh` _output_get_2) (`/Game/_Main/Player/BP_Player.FPSArms` _player_referance) (`/Game/_Main/Weapon/BP_EQ_WeaponBase.AttachSocket` _output_get_2) "SnapToTarget" "SnapToTarget" "SnapToTarget" true)
        (message `/Game/_Main/Interfaces/INT_Player.LevelReset` _player_referance_2))
      (:`else`
        (`KismetSystemLibrary.Delay` 0.2)
        (goto _label)))))

(event `self.ReceiveBeginPlay`
  (bind _outactors (`GameplayStatics.GetAllActorsOfClass` "/Game/_Main/Game/BP_LevelType.BP_LevelType_C"))
  (bind _output (`|GetArrayItem` _outactors))
  (set `self.Level Type` (`/Game/_Main/Game/BP_LevelType.LevelType` _output))
  (set `self.Next Level Name` (`/Game/_Main/Game/BP_LevelType.NextLevelName` _output))
  (set `self.Has Timer` (`/Game/_Main/Game/BP_LevelType.HasTimer` _output))
  (set `self.Level Time` (`/Game/_Main/Game/BP_LevelType.LevelTime` _output))
  (`self.LoadPlayerData`)
  (if (`self.Has Timer`)
    (bind _returnvalue (`KismetSystemLibrary.K2_SetTimerDelegate` (delegate `LevelCountdownTimer`) 1.0 true))
    (set `self.LevelTimerHandle` _returnvalue)))

(event `LevelCountdownTimer`
  (bind _player_controller (`self.Player Controller`))
  (bind _player_controller_2 (`self.Player Controller`)
    (:`then`
      (`self.F_HandleLevelTimer`)
      (message `/Game/_Main/Interfaces/INT_PlayerController.UpdateLevelText` _player_controller_2 (`self.Result`))
      (if (<= (`self.Level Time`) 0.0)
        (message `/Game/_Main/Interfaces/INT_PlayerController.ShowPlayerDeathScreen` _player_controller)
        (bind _playerreferance (message `/Game/_Main/Interfaces/INT_Player.GetPlayerReferance` (`Controller.K2_GetPawn` _player_controller)))
        (set `/Game/_Main/BP_BaseCharacter.IsDead` true _playerreferance)
        (`self.ClearLevelTimer`)))
    (:`else`)))

(event `/Game/_Main/Interfaces/INT_GameMode.AddEnemy`
  (params (Enemy :type "Actor Object Reference"))
  (`KismetArrayLibrary.Array_AddUnique` (`self.EnemyList`) Enemy)
  (add `self.OnDestroyed` Enemy (delegate `RemoveEnemy`))
  (bind _enemybasereferance (message `/Game/_Main/Interfaces/INT_EnemyCharacter.GetEnemyCharacterReferance` Enemy))
  (`/Engine/EditorBlueprintResources/StandardMacros.IsValid` _enemybasereferance
    (:`Is Valid`
      (add `/Game/_Main/Enemies/Humanoid/BP_EnemyBase.EnemyKilled` _enemybasereferance (delegate `CustomEvent`)))))

(event `CustomEvent`
  (params (EnemyRemoved :type "Actor Object Reference"))
  (`/Engine/EditorBlueprintResources/StandardMacros.IsValid` EnemyRemoved
    (:`Is Valid`
      (if (> (`KismetArrayLibrary.Array_Find` (`self.EnemyList`) EnemyRemoved) -1)
        (`KismetArrayLibrary.Array_RemoveItem` (`self.EnemyList`) EnemyRemoved)
        (if (== (`KismetArrayLibrary.Array_Length` (`self.EnemyList`)) 0) :!label _label_2
          (switch `/Game/_Main/Game/E_LevelType` (`self.Level Type`)
            (:`NewEnumerator0`
              (`self.SaveGame`)
              (`self.ClearLevelTimer`)
              (`GameplayStatics.OpenLevel` (`KismetStringLibrary.Conv_StringToName` (`KismetStringLibrary.Concat_StrStr` "/Game/_Main/Maps/" (`self.Next Level Name`)))))))))))

(event `RemoveEnemy` :!signature `self.OnDestroyed`
  (params (DestroyedActor :type "Actor Object Reference"))
  (`/Engine/EditorBlueprintResources/StandardMacros.IsValid` DestroyedActor
    (:`Is Valid`
      (if (> (`KismetArrayLibrary.Array_Find` (`self.EnemyList`) DestroyedActor) -1)
        (`KismetArrayLibrary.Array_RemoveItem` (`self.EnemyList`) DestroyedActor)
        (goto _label_2)))))

(event `/Game/_Main/Interfaces/INT_GameMode.EndOfLevelReached`
  (switch `/Game/_Main/Game/E_LevelType` (`self.Level Type`)
    (:`NewEnumerator1`
      (`self.SaveGame`)
      (`self.ClearLevelTimer`)
      (`GameplayStatics.OpenLevel` (`KismetStringLibrary.Conv_StringToName` (`KismetStringLibrary.Concat_StrStr` "/Game/_Main/Maps/" (`self.Next Level Name`)))))))

(event `/Game/_Main/Interfaces/INT_GameMode.AddPlayerControllerToGameMode`
  (params (PlayerController :type "PlayerController Object Reference"))
  (set `self.Player Controller` PlayerController))

(event `ClearLevelTimer`
  (`KismetSystemLibrary.K2_ClearAndInvalidateTimerHandle` (`self.LevelTimerHandle`)))

(event `SaveGame`
  (bind _player_referance (`self.Player Referance`))
  (bind _player_controller (`self.Player Controller`)
    (:`then`
      (bind _playerreferance (message `/Game/_Main/Interfaces/INT_Player.GetPlayerReferance` (`Controller.K2_GetPawn` _player_controller)))
      (bind _output_get (set `self.Player Referance` _playerreferance))
      (`/Engine/EditorBlueprintResources/StandardMacros.IsValid` _output_get
        (:`Is Valid`
          (bind _returnvalue (`GameplayStatics.CreateSaveGameObject` "/Game/_Main/SG_GameSave.SG_GameSave_C"))
          (bind _output_get_2 (set `self.SaveGameInfo` _returnvalue))
          (set `/Game/_Main/SG_GameSave.CurrentlyHeldWeapon` (`GameplayStatics.GetObjectClass` (`/Game/_Main/Player/BP_Player.HeldWeapon` _player_referance)) _output_get_2)
          (set `/Game/_Main/SG_GameSave.PickedUpItems` (`/Game/_Main/Player/BP_Player.PickedUpItems` _player_referance) _output_get_2)
          (set `/Game/_Main/SG_GameSave.OwnedWeapons` (`/Game/_Main/Player/BP_Player.OwnedWeapons` _player_referance) _output_get_2)
          (set `/Game/_Main/SG_GameSave.CurrentAmmo` (`/Game/_Main/Player/BP_Player.OwnedWeaponCurrentAmmo` _player_referance) _output_get_2)
          (set `/Game/_Main/SG_GameSave.TotalAmmo` (`/Game/_Main/Player/BP_Player.OwnedWeaponTotalAmmo` _player_referance) _output_get_2)
          (set `/Game/_Main/SG_GameSave.LevelName` (`self.Next Level Name`) _output_get_2)
          (bind _savegamename (message `/Game/_Main/Interfaces/INT_GameInstance.GetSaveGameName` (`GameplayStatics.GetGameInstance`)))
          (`GameplayStatics.SaveGameToSlot` (`self.SaveGameInfo`) _savegamename))
        (:`Is Not Valid`
          (`KismetSystemLibrary.PrintString` "Invalid Character"))))
    (:`else`
      (`KismetSystemLibrary.PrintString` "Could Not get data"))))

(event `/Game/_Main/Interfaces/INT_GameMode.LoadGame`
  (bind _player_referance (`self.Player Referance`))
  (bind _player_controller (`self.Player Controller`)
    (:`then`
      (bind _playerreferance (message `/Game/_Main/Interfaces/INT_Player.GetPlayerReferance` (`Controller.K2_GetPawn` _player_controller)))
      (set `self.Player Referance` _playerreferance)
      (bind _savegamename (message `/Game/_Main/Interfaces/INT_GameInstance.GetSaveGameName` (`GameplayStatics.GetGameInstance`)))
      (bind _returnvalue (`GameplayStatics.DoesSaveGameExist` _savegamename))
      (if _returnvalue
        (bind _returnvalue_2 (`GameplayStatics.LoadGameFromSlot` _savegamename))
        (bind _output_get (set `self.LoadGameData` (cast `/Game/_Main/SG_GameSave` _returnvalue_2 :!pure true)))
        (set `/Game/_Main/Player/BP_Player.OwnedWeaponCurrentAmmo` (`/Game/_Main/SG_GameSave.CurrentAmmo` _output_get) _player_referance)
        (set `/Game/_Main/Player/BP_Player.OwnedWeaponTotalAmmo` (`/Game/_Main/SG_GameSave.TotalAmmo` _output_get) _player_referance)
        (set `/Game/_Main/Player/BP_Player.OwnedWeapons` (`/Game/_Main/SG_GameSave.OwnedWeapons` _output_get) _player_referance)
        (else
          (`KismetSystemLibrary.PrintString` "NO SAVE GAME"))))
    (:`else`)))

(fn `F_HandleLevelTimer`
  (bind _returnvalue (mod (`self.Level Time`) 60.0))
  (bind _returnvalue_2 (`KismetMathLibrary.FFloor` (/ (`self.Level Time`) 60.0)))
  (`/Engine/EditorBlueprintResources/StandardMacros.DecrementFloat` (`self.Level Time`)
    (:`  `
      (if (< _returnvalue 10.0)
        (set `self.Result` (`|FormatText` "{MIN}:0{SECOUNDS}" _returnvalue_2 _returnvalue))
        (else
          (set `self.Result` (`|FormatText` "{MIN}:{SECOUNDS}" _returnvalue_2 _returnvalue))))
      (return))))

(fn `UserConstructionScript`)