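; First-person player character Blueprint handling weapons, health, death, pickups and interaction with doors, buttons and levers.
; Firing uses camera line traces with a delay loop for automatic weapons; reloads apply when the arms montage completes.
; Owned weapon classes key the magazine and reserve ammo maps, so switching destroys and respawns the held weapon without losing ammo.
; Health, ammo, interact prompts and death screen go through PlayerController; picked-up items unlock gated interactables.
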(event `self.ReceiveBeginPlay`
  (`parent.ReceiveBeginPlay`)
  (set `self.CurrentHealth` (`self.MaxHealth`))
  (`self.F_UpdateHealth`))

(event `self.ReceivePossessed`
  (params (NewController :type "Controller Object Reference"))
  (set `self.PlayerController` NewController))

(event `EnhancedInput|/Game/_Main/Inputs/InputActions/IA_FireWeapon`
  (params (ActionValue :type Boolean) (ElapsedSeconds :type "Float (double-precision)") (TriggeredSeconds :type "Float (double-precision)") (InputAction :type "InputAction Object Reference" :default "/Game/_Main/Inputs/InputActions/IA_FireWeapon.IA_FireWeapon"))
  (bind _returnvalue (`GameplayStatics.GetPlayerCameraManager` 0))
  (bind _ownedweaponcurrentammo (`self.OwnedWeaponCurrentAmmo`))
  (bind _heldweapon (`self.HeldWeapon`))
  (bind _returnvalue_2 (`self.K2_GetActorLocation` _returnvalue))
  (bind _returnvalue_3 (`GameplayStatics.GetObjectClass` (`self.HeldWeapon`)))
  (bind _muzzleflashpoint (`/Game/_Main/Weapon/BP_EQ_WeaponBase.MuzzleFlashPoint` _heldweapon))
  (:`Started`
    (set `self.FireButtonHeld` true)
    (if (and (not (`self.IsReloading`)) (not (`self.IsDead`)))
      (bind _heldweapon_2 (`self.HeldWeapon`)
        (:`then`
          (if (> (`BlueprintMapLibrary.Map_Find` (`self.OwnedWeaponCurrentAmmo`) (`GameplayStatics.GetObjectClass` _heldweapon_2)) 0) :!label _label
            (`BlueprintMapLibrary.Map_Add` _ownedweaponcurrentammo _returnvalue_3 (- (`BlueprintMapLibrary.Map_Find` _ownedweaponcurrentammo _returnvalue_3) 1))
            (`self.F_UpdateAmmo`)
            (`GameplayStatics.SpawnEmitterAtLocation` (`/Game/_Main/Weapon/BP_EQ_WeaponBase.MuzleFlash` _heldweapon) (`SceneComponent.K2_GetComponentLocation` _muzzleflashpoint) (`SceneComponent.K2_GetComponentRotation` _muzzleflashpoint) (0.05 0.05 0.05))
            (`GameplayStatics.PlaySound2D` (`/Game/_Main/Weapon/BP_EQ_WeaponBase.FireWeapom` (`self.HeldWeapon`)) 1.0 1.0 0.0 null null)
            (bind (_outhit _returnvalue_4) (`KismetSystemLibrary.LineTraceSingle` :`Start` _returnvalue_2 :`End` (+ _returnvalue_2 (* (`self.GetActorForwardVector` _returnvalue) (`/Game/_Main/Weapon/BP_EQ_WeaponBase.FireDistance` (`self.HeldWeapon`)))) :`TraceChannel` "TraceTypeQuery1" :`DrawDebugType` "ForDuration" :`DrawTime` 10.0))
            (if _returnvalue_4
              (`GameplayStatics.ApplyDamage` (`.HitActor` (`GameplayStatics.BreakHitResult` _outhit)) (`/Game/_Main/Weapon/BP_EQ_WeaponBase.Damage` (`self.HeldWeapon`))))
            (if (`/Game/_Main/Weapon/BP_EQ_WeaponBase.Automatic` (`self.HeldWeapon`))
              (`KismetSystemLibrary.Delay` (`/Game/_Main/Weapon/BP_EQ_WeaponBase.FireRate` (`self.HeldWeapon`)))
              (if (`self.FireButtonHeld`)
                (goto _label)))
            (else
              (`GameplayStatics.PlaySound2D` (`/Game/_Main/Weapon/BP_EQ_WeaponBase.OutOfAmmo` (`self.HeldWeapon`)) 1.0 1.0 0.0 null null))))
        (:`else`))))
  (:`Canceled`
    (set `self.FireButtonHeld` false :!label _label_2)
    (set `self.FireButtonRelease` true))
  (:`Completed`
    (goto _label_2)))

(event `/Game/_Main/Interfaces/INT_Player.PlayerOverlapsWeapon`
  (params (OverlappedWeapon :type "/Game/_Main/Weapon/BP_WeaponPickupBase Object Reference"))
  (bind _heldweapon (`self.HeldWeapon`))
  (if (not (`self.IsDead`))
    (`self.HeldWeapon`
      (:`then`
        (bind _returnvalue (`KismetArrayLibrary.Array_AddUnique` (`self.OwnedWeapons`) (`/Game/_Main/Weapon/BP_WeaponPickupBase.EquipClass` OverlappedWeapon)))
        (if (< _returnvalue 0)
          (bind _shouldpickup (`self.F_PickupOwnedWeapon` OverlappedWeapon))
          (if _shouldpickup
            (`self.K2_DestroyActor` OverlappedWeapon)
            (`self.F_UpdateAmmo`))
          (else
            (`self.F_PickupNewWeaponWhileHolding` OverlappedWeapon)
            (`self.K2_DestroyActor` OverlappedWeapon))))
      (:`else`
        (`self.F_FirstWeaponPickup` OverlappedWeapon)
        (bind _returnvalue_2 (`|SpawnActorFromClass` (`/Game/_Main/Weapon/BP_WeaponPickupBase.EquipClass` OverlappedWeapon) (`KismetMathLibrary.MakeTransform` (`self.K2_GetActorLocation`)) "AdjustIfPossibleButAlwaysSpawn" "MultiplyWithRoot" null null))
        (set `self.HeldWeapon` _returnvalue_2)
        (`self.F_UpdateAmmo`)
        (`SceneComponent.K2_AttachToComponent` (`/Game/_Main/Weapon/BP_EQ_WeaponBase.SkeletalMesh` _heldweapon) (`self.FPSArms`) (`/Game/_Main/Weapon/BP_EQ_WeaponBase.AttachSocket` _heldweapon) "SnapToTarget" "SnapToTarget" "KeepRelative" true)
        (`self.K2_DestroyActor` OverlappedWeapon)))))

(event `EnhancedInput|/Game/_Main/Inputs/InputActions/IA_Reload`
  (params (ActionValue :type Boolean) (ElapsedSeconds :type "Float (double-precision)") (TriggeredSeconds :type "Float (double-precision)") (InputAction :type "InputAction Object Reference" :default "/Game/_Main/Inputs/InputActions/IA_Reload.IA_Reload"))
  (bind _heldweapon (`self.HeldWeapon`))
  (:`Started`
    (if (and (not (`self.IsDead`)) (not (`self.FireButtonHeld`)))
      (if (not (== (`/Game/_Main/Weapon/BP_EQ_WeaponBase.MaxMagAmmo` _heldweapon) (`BlueprintMapLibrary.Map_Find` (`self.OwnedWeaponCurrentAmmo`) (`GameplayStatics.GetObjectClass` _heldweapon))))
        (if (> (`BlueprintMapLibrary.Map_Find` (`self.OwnedWeaponTotalAmmo`) (`GameplayStatics.GetObjectClass` (`self.HeldWeapon`))) 0)
          (if (not (`self.IsReloading`))
            (set `self.IsReloading` true)
            (`|PlayMontage` (`self.FPSArms`) (`/Game/_Main/Weapon/BP_EQ_WeaponBase.ReloadMontage` (`self.HeldWeapon`))
              (:`then`
                (`GameplayStatics.PlaySound2D` (`/Game/_Main/Weapon/BP_EQ_WeaponBase.ReloadWeapon` (`self.HeldWeapon`)) 1.0 1.0 0.0 null null))
              (:`OnCompleted`
                (`self.F_Reload`)
                (set `self.IsReloading` false)
                (`self.F_UpdateAmmo`))))
          (else
            (`KismetSystemLibrary.PrintString` "No Ammo left")))
        (else
          (`KismetSystemLibrary.PrintString` "Mag Full"))))))

(event `self.ReceiveAnyDamage`
  (params (Damage :type "Float (single-precision)") (DamageType :type "DamageType Object Reference") (InstigatedBy :type "Controller Object Reference") (DamageCauser :type "Actor Object Reference"))
  (set `self.CurrentHealth` (`KismetMathLibrary.FClamp` (- (`self.CurrentHealth`) Damage) 0.0 (`self.MaxHealth`)))
  (`self.F_UpdateHealth`)
  (if (== (`self.CurrentHealth`) 0.0)
    (if (not (`self.IsDead`))
      (`self.HandlePlayerDeath`))))

(event `HandlePlayerDeath`
  (set `self.IsDead` true)
  (message `/Game/_Main/Interfaces/INT_PlayerController.ShowPlayerDeathScreen` (`self.PlayerController`)))

(event `/Game/_Main/Interfaces/INT_Player.SetInteractObject`
  (params (overlappedInteractable :type "/Game/_Main/Interactable/BP_InteractableBase Object Reference"))
  (`self.PlayerController`
    (:`then`
      (bind _output_get (set `self.Overlapped Interactable` overlappedInteractable))
      (`/Engine/EditorBlueprintResources/StandardMacros.IsValid` _output_get
        (:`Is Valid`
          (if (not (`self.IsDead`))
            (message `/Game/_Main/Interfaces/INT_PlayerController.SetInteractText` (`self.PlayerController`) (`|FormatText` "Press \"E\" to use {interactableName}" (`/Game/_Main/Interactable/BP_InteractableBase.InterectName` _output_get)) "Visible")))
        (:`Is Not Valid`
          (message `/Game/_Main/Interfaces/INT_PlayerController.SetInteractText` (`self.PlayerController`) "" "Hidden"))))
    (:`else`)))

(event `EnhancedInput|/Game/_Main/Inputs/InputActions/IA_Interact`
  (params (ActionValue :type Boolean) (ElapsedSeconds :type "Float (double-precision)") (TriggeredSeconds :type "Float (double-precision)") (InputAction :type "InputAction Object Reference" :default "/Game/_Main/Inputs/InputActions/IA_Interact.IA_Interact"))
  (:`Started`
    (if (and (not (`self.IsDead`)) (not (`self.IsReloading`)))
      (bind _overlapped_interactable (`self.Overlapped Interactable`)
        (:`then`
          (if (not (`/Game/_Main/Interactable/BP_InteractableBase.RequiredItemsToOpen` _overlapped_interactable))
            (switch `/Game/_Main/Interactable/E_InteractType` (`/Game/_Main/Interactable/BP_InteractableBase.InterectType` _overlapped_interactable) :!label _label_3
              (:`NewEnumerator0`
                (`|PlayMontage` (`self.FPSArms`) "/Game/_Main/Player/Player_OpenDoor_Montage.Player_OpenDoor_Montage" :!label _label_4
                  (:`then`
                    _)))
              (:`NewEnumerator1`
                (goto _label_4))
              (:`NewEnumerator3`
                _))
            (`/Game/_Main/Interactable/BP_InteractableBase.UseInteractable` (`self.Overlapped Interactable`))
            (else
              (for _array_element (`self.PickedUpItems`)
                (bind _itemsrequired (`/Game/_Main/Interactable/BP_InteractableBase.ItemsRequired` _overlapped_interactable))
                (if (== _array_element _itemsrequired)
                  (`KismetArrayLibrary.Array_RemoveItem` (`self.PickedUpItems`) _itemsrequired)
                  (goto _label_3))))))
        (:`else`)))))

(event `/Game/_Main/Interfaces/INT_Player.HandlePickup`
  (params (OverlappedPickup :type "/Game/_Main/PickUps/BP_BasePickup Object Reference"))
  (if (not (`self.IsDead`))
    (bind _output_get (set `self.Overlapped Pickup` OverlappedPickup))
    (switch `/Game/_Main/PickUps/E_PickupType` (`/Game/_Main/PickUps/BP_BasePickup.PickupType` _output_get)
      (:`NewEnumerator0`
        (`self.F_PickupHealth`))
      (:`NewEnumerator1`
        (`KismetArrayLibrary.Array_AddUnique` (`self.PickedUpItems`) (`GameplayStatics.GetObjectClass` OverlappedPickup))
        (`self.K2_DestroyActor` (`self.Overlapped Pickup`))))))

(event `EnhancedInput|/Game/_Main/Inputs/InputActions/IA_SwitchWeapon`
  (params (ActionValue :type "Float (double-precision)") (ElapsedSeconds :type "Float (double-precision)") (TriggeredSeconds :type "Float (double-precision)") (InputAction :type "InputAction Object Reference" :default "/Game/_Main/Inputs/InputActions/IA_SwitchWeapon.IA_SwitchWeapon"))
  (bind _heldweapon (`self.HeldWeapon`))
  (:`Triggered`
    (if (not (`self.IsReloading`))
      (`self.HeldWeapon`
        (:`then`
          (bind _foundweapontospawn (`self.F_SwitchWeaponLogic` ActionValue))
          (if _foundweapontospawn
            (bind _nextweapontospawn (`self.NextWeaponToSpawn`)
              (:`then`
                (bind _returnvalue (`|SpawnActorFromClass` _nextweapontospawn (`KismetMathLibrary.MakeTransform` (`self.K2_GetActorLocation`)) "AlwaysSpawn" "MultiplyWithRoot" null null))
                (`self.K2_DestroyActor` (`self.HeldWeapon`))
                (set `self.HeldWeapon` _returnvalue)
                (`SceneComponent.K2_AttachToComponent` (`/Game/_Main/Weapon/BP_EQ_WeaponBase.SkeletalMesh` _heldweapon) (`self.FPSArms`) (`/Game/_Main/Weapon/BP_EQ_WeaponBase.AttachSocket` _heldweapon) "SnapToTarget" "SnapToTarget" "KeepRelative" true)
                (`self.F_UpdateAmmo`))
              (:`else`))))
        (:`else`)))))

(fn `F_FirstWeaponPickup`
  (params (OverLappedWeapon :type "/Game/_Main/Weapon/BP_WeaponPickupBase Object Reference"))
  (bind _equipclass (`/Game/_Main/Weapon/BP_WeaponPickupBase.EquipClass` OverLappedWeapon))
  (bind _newpickupammo (`/Game/_Main/Weapon/BP_WeaponPickupBase.NewPickupAmmo` OverLappedWeapon))
  (bind _maxmagammo (`/Game/_Main/Weapon/BP_WeaponPickupBase.MaxMagAmmo` OverLappedWeapon))
  (bind _ownedweaponcurrentammo (`self.OwnedWeaponCurrentAmmo`))
  (bind _ownedweapontotalammo (`self.OwnedWeaponTotalAmmo`))
  (`KismetArrayLibrary.Array_AddUnique` (`self.OwnedWeapons`) _equipclass)
  (if (> _newpickupammo _maxmagammo)
    (`BlueprintMapLibrary.Map_Add` _ownedweaponcurrentammo _equipclass _maxmagammo)
    (`BlueprintMapLibrary.Map_Add` _ownedweapontotalammo _equipclass (- _newpickupammo _maxmagammo))
    (else
      (`BlueprintMapLibrary.Map_Add` _ownedweaponcurrentammo _equipclass _newpickupammo)
      (`BlueprintMapLibrary.Map_Add` _ownedweapontotalammo _equipclass)))
  (return))

(fn `F_PickupHealth`
  (if (!= (`self.CurrentHealth`) (`self.MaxHealth`))
    (bind _healthtoadd (message `/Game/_Main/Interfaces/INT_Pickup.GetHealthToAdd` (`self.Overlapped Pickup`)))
    (set `self.CurrentHealth` (`KismetMathLibrary.FClamp` (+ (`self.CurrentHealth`) _healthtoadd) 0.0 (`self.MaxHealth`)))
    (`self.F_UpdateHealth`)
    (`self.K2_DestroyActor` (`self.Overlapped Pickup`))))

(fn `F_PickupNewWeaponWhileHolding`
  (params (OverLappedWeapon :type "/Game/_Main/Weapon/BP_WeaponPickupBase Object Reference"))
  (bind _equipclass (`/Game/_Main/Weapon/BP_WeaponPickupBase.EquipClass` OverLappedWeapon))
  (bind _newpickupammo (`/Game/_Main/Weapon/BP_WeaponPickupBase.NewPickupAmmo` OverLappedWeapon))
  (bind _maxmagammo (`/Game/_Main/Weapon/BP_WeaponPickupBase.MaxMagAmmo` OverLappedWeapon))
  (bind _ownedweaponcurrentammo (`self.OwnedWeaponCurrentAmmo`))
  (bind _ownedweapontotalammo (`self.OwnedWeaponTotalAmmo`))
  (if (> _newpickupammo _maxmagammo)
    (`BlueprintMapLibrary.Map_Add` _ownedweaponcurrentammo _equipclass _maxmagammo)
    (`BlueprintMapLibrary.Map_Add` _ownedweapontotalammo _equipclass (- _newpickupammo _maxmagammo))
    (else
      (`BlueprintMapLibrary.Map_Add` _ownedweaponcurrentammo _equipclass _newpickupammo)
      (`BlueprintMapLibrary.Map_Add` _ownedweapontotalammo _equipclass)))
  (return))

(fn `F_PickupOwnedWeapon`
  (params (OverLappedWeapon :type "/Game/_Main/Weapon/BP_WeaponPickupBase Object Reference"))
  (returns (ShouldPickup :type Boolean))
  (bind _equipclass (`/Game/_Main/Weapon/BP_WeaponPickupBase.EquipClass` OverLappedWeapon))
  (bind _maxtotalammo (`/Game/_Main/Weapon/BP_WeaponPickupBase.MaxTotalAmmo` OverLappedWeapon))
  (bind _value (`BlueprintMapLibrary.Map_Find` (`self.OwnedWeaponTotalAmmo`) _equipclass))
  (if (not (== _maxtotalammo _value))
    (`BlueprintMapLibrary.Map_Add` (`self.OwnedWeaponTotalAmmo`) _equipclass (`KismetMathLibrary.Clamp` (+ _value (`/Game/_Main/Weapon/BP_WeaponPickupBase.PickupAmmo` OverLappedWeapon)) 0 _maxtotalammo))
    (return true)
    (else
      (return false))))

(fn `F_Reload`
  (bind _heldweapon (`self.HeldWeapon`))
  (bind _returnvalue (`GameplayStatics.GetObjectClass` (`self.HeldWeapon`)))
  (bind _returnvalue_2 (`GameplayStatics.GetObjectClass` (`self.HeldWeapon`)))
  (bind _returnvalue_3 (`GameplayStatics.GetObjectClass` _heldweapon))
  (bind _returnvalue_4 (- (`/Game/_Main/Weapon/BP_EQ_WeaponBase.MaxMagAmmo` _heldweapon) (`BlueprintMapLibrary.Map_Find` (`self.OwnedWeaponCurrentAmmo`) _returnvalue_3)))
  (if (>= (`BlueprintMapLibrary.Map_Find` (`self.OwnedWeaponTotalAmmo`) _returnvalue_3) _returnvalue_4)
    (`BlueprintMapLibrary.Map_Add` (`self.OwnedWeaponTotalAmmo`) _returnvalue_2 (- (`BlueprintMapLibrary.Map_Find` (`self.OwnedWeaponTotalAmmo`) (`GameplayStatics.GetObjectClass` (`self.HeldWeapon`))) _returnvalue_4))
    (`BlueprintMapLibrary.Map_Add` (`self.OwnedWeaponCurrentAmmo`) _returnvalue_2 (`/Game/_Main/Weapon/BP_EQ_WeaponBase.MaxMagAmmo` (`self.HeldWeapon`)))
    (else
      (`BlueprintMapLibrary.Map_Add` (`self.OwnedWeaponCurrentAmmo`) _returnvalue (+ (`BlueprintMapLibrary.Map_Find` (`self.OwnedWeaponCurrentAmmo`) _returnvalue) (`BlueprintMapLibrary.Map_Find` (`self.OwnedWeaponTotalAmmo`) _returnvalue)))
      (`BlueprintMapLibrary.Map_Add` (`self.OwnedWeaponTotalAmmo`) _returnvalue)))
  (return))

(fn `F_SwitchWeaponLogic`
  (params (SwitchDirections :type "Float (double-precision)"))
  (returns (FoundWeaponToSpawn :type Boolean))
  (locals (UseNext :type Boolean) (NextWeaponFound :type Boolean))
  (set `local.UseNext` false)
  (set `local.NextWeaponFound` false)
  (set `self.NextWeaponToSpawn` null)
  (if (> SwitchDirections 0.0)
    (for _array_element (`self.OwnedWeapons`)
      (if (== _array_element (`GameplayStatics.GetObjectClass` (`self.HeldWeapon`)))
        (set `local.UseNext` true)
        (elif (`local.UseNext`)
          (set `local.UseNext` false)
          (set `self.NextWeaponToSpawn` _array_element)
          (set `local.NextWeaponFound` true))))
    (return (`local.NextWeaponFound`))
    (else
      (bind (_arrayindex _arrayelement) (`/Engine/EditorBlueprintResources/StandardMacros.ReverseForEachLoop` (`self.OwnedWeapons`))
        (:`LoopBody`
          (if (== _arrayelement (`GameplayStatics.GetObjectClass` (`self.HeldWeapon`)))
            (set `local.UseNext` true)
            (elif (`local.UseNext`)
              (set `local.UseNext` false)
              (set `self.NextWeaponToSpawn` _arrayelement)
              (set `local.NextWeaponFound` true))))
        (:`Completed`
          (return (`local.NextWeaponFound`)))))))

(fn `F_UpdateAmmo`
  (bind _heldweapon (`self.HeldWeapon`))
  (bind _returnvalue (`GameplayStatics.GetObjectClass` _heldweapon))
  (message `/Game/_Main/Interfaces/INT_PlayerController.UpdateAmmoUI` (`self.PlayerController`) (`/Game/_Main/Weapon/BP_EQ_WeaponBase.WeaponName` _heldweapon) (`BlueprintMapLibrary.Map_Find` (`self.OwnedWeaponCurrentAmmo`) _returnvalue) (`BlueprintMapLibrary.Map_Find` (`self.OwnedWeaponTotalAmmo`) _returnvalue)))

(fn `F_UpdateHealth`
  (message `/Game/_Main/Interfaces/INT_PlayerController.UpdateHealthUI` (`self.PlayerController`) (/ (`self.CurrentHealth`) (`self.MaxHealth`))))

(fn `GetPlayerReferance`
  (returns (PlayerReferance :type "/Game/_Main/Player/BP_Player Object Reference"))
  (return self))

(fn `UserConstructionScript`
  (`parent.UserConstructionScript`))